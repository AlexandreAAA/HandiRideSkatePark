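; Player skateboarder character that starts in a custom Skate movement mode, with impulse-based pushing and ollie, and turn input fed to ABP_Skater.
; Tick aligns camera yaw to actual travel direction, moves the board between capsule and hand socket for Christ Air grabs, and crashes on landing off-board.
; Overlapping a BP_GrindableObstacle captures speed and rail spline data for grinding.
; Comments place grind movement and flatground gesture tricks in C++.
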(event Input|EnhancedActionEvents|EnhancedInputActionIA_Move
  (params (ActionValue :type Vector%202D%20Structure) (ElapsedSeconds :type Float%20%28double-precision%29) (TriggeredSeconds :type Float%20%28double-precision%29) (InputAction :type Input%20Action%20Object%20Reference :default "/Game/ThirdPerson/Input/Actions/IA_Move.IA_Move"))
  (bind _mesh (Variables|Character|GetMesh))
  (bind _returnvalue (Components|SkeletalMesh|GetAnimInstance _mesh))
  (:Triggered
    (bind _asabp_skater (Utilities|Casting|CastToABP_Skater _returnvalue))
    (Variables|/Game/SkateAssets/Animations/ABP_Skater.ABP_Skater_C|SetTurnInput _asabp_skater (.x ActionValue)))
  (:Completed
    (bind _asabp_skater_2 (Utilities|Casting|CastToABP_Skater _returnvalue))
    (Variables|/Game/SkateAssets/Animations/ABP_Skater.ABP_Skater_C|SetTurnInput _asabp_skater_2 0.0)))

(event Input|EnhancedActionEvents|EnhancedInputActionIA_MoveFwd
  (params (ActionValue :type Float%20%28double-precision%29) (ElapsedSeconds :type Float%20%28double-precision%29) (TriggeredSeconds :type Float%20%28double-precision%29) (InputAction :type Input%20Action%20Object%20Reference :default "/Game/ThirdPerson/Input/Actions/IA_MoveFwd.IA_MoveFwd"))
  ;[1 1 1] Pushing
  (bind _asskate_character_movement_component (Utilities|Casting|CastToSkateCharacterMovementComponent (Variables|Character|GetCharacterMovement)))
  (if (Class|SkateCharacterMovementComponent|IsCustomMovementMode _asskate_character_movement_component "CMOVE_Skate")
    (Physics|AddImpulse (Variables|Character|GetCharacterMovement) (* (* (Math|Vector|GetForwardVector (Variables|Default|GetCapsuleComponent)) ActionValue) 5.0) true)))

(event EventBeginPlay
  (Utilities|FlowControl|Sequence
    (:then_0
      (Pawn|Components|CharacterMovement|SetMovementMode (Variables|Character|GetCharacterMovement) "MOVE_Custom" (Utilities|Enum|LiteralenumECustomMovementMode "CMOVE_Skate")))
    (:then_1
      (Variables|Default|SetSkateboardRidingTransform (Transformation|GetRelativeTransform (Variables|Default|GetSkateboardMesh))))))

(event EventOnOverlapCheckGrind
  (params (OverlappedComp :type Primitive%20Component%20Object%20Reference) (OtherActor :type Actor%20Object%20Reference) (OtherComp :type Primitive%20Component%20Object%20Reference) (OtherBodyIndex :type Integer) (bFromSweep :type Boolean) (SweepResult :type Hit%20Result%20Structure%20%28by%20ref%29))
  ;[1 1 1] Grnding data retreived in Blueprint via BP_Grindable object  ; grind movement computed in CPP
  (if (not (Variables|Default|Get_isGrinding))
    (bind _asbp_grindable_obstacle (Utilities|Casting|CastToBP_GrindableObstacle OtherActor))
    (Variables|Default|SetGrindingSpeed (Math|Vector|VectorLengthXY (Variables|/Script/Engine.MovementComponent|GetVelocity (Variables|Character|GetCharacterMovement)))) ; Set grind speed based on prev speed
    (Variables|Default|Set_isGrinding true)
    (bind (_distancealongspline _directionscalar _railheightoffset) (Default|GetGrindInfo _asbp_grindable_obstacle self))
    (Variables|Default|SetDistanceAlongRail _distancealongspline)
    (Variables|Default|SetRailDirectionScalar _directionscalar)
    (Variables|Default|SetRailHeightOffset _railheightoffset)
    (Variables|Default|SetcurrentRail (Variables|/Game/SkateAssets/BP_GrindableObstacle.BP_GrindableObstacle_C|GetGrindSpline _asbp_grindable_obstacle))))

(event EventTick
  (params (DeltaSeconds :type Float%20%28single-precision%29))
  (bind _skateboardmesh (Variables|Default|GetSkateboardMesh))
  ;[1 1 1] Align camera
  (Utilities|FlowControl|Sequence ; Then 2 in Crash
    (:then_0
      (bind _asskate_character_movement_component (Utilities|Casting|CastToSkateCharacterMovementComponent (Variables|Character|GetCharacterMovement)))
      (if (Class|SkateCharacterMovementComponent|IsCustomMovementMode _asskate_character_movement_component "CMOVE_Skate")
        (CallFunction|AlignCamerawithMoveDirection)))
    (:then_1
      ;[1 1 1] Christ Air Hold Board
      (bind _asskate_character_movement_component_2 (Utilities|Casting|CastToSkateCharacterMovementComponent (Variables|Character|GetCharacterMovement)))
      (if (Class|SkateCharacterMovementComponent|IsCustomMovementMode _asskate_character_movement_component_2 "CMOVE_Skate")
        (if (and (Variables|Grabs|GetisChristAir) (Variables|Grabs|GetisRightGrab))
          (if (Variables|Default|GetisOnBoard?)
            (Transformation|AttachComponentToComponent (Variables|Default|GetSkateboardMesh) (Variables|Character|GetMesh) "SkateboardSocket" "SnapToTarget" "SnapToTarget" "KeepWorld" false)
            (Variables|Default|SetisOnBoard? false))
          (elif (not (Variables|Default|GetisOnBoard?))
            (Transformation|AttachComponentToComponent _skateboardmesh (Variables|Default|GetCapsuleComponent) "" "SnapToTarget" "SnapToTarget" "SnapToTarget" false)
            (Transformation|SetRelativeTransform _skateboardmesh (Variables|Default|GetSkateboardRidingTransform) false false)
            (Variables|Default|SetisOnBoard? true)))))
    (:then_2
      ;[1 1 1] CRASH if we land and were not on the board
      (bind _asskate_character_movement_component_3 (Utilities|Casting|CastToSkateCharacterMovementComponent (Variables|Character|GetCharacterMovement)))
      (if (Class|SkateCharacterMovementComponent|IsCustomMovementMode _asskate_character_movement_component_3 "CMOVE_Skate")
        (if (and (not (Variables|Default|GetisOnBoard?)) (not (Variables|/Script/PPPSkateboard.SkateCharacterMovementComponent|GetisAerial _asskate_character_movement_component_3)))
          (Class|SkateCharacter|Crash))))))

(event Input|KeyboardEvents|SpaceBar
  (params (Key :type Key%20Structure :default "None"))
  (bind _charactermovement (Variables|Character|GetCharacterMovement))
  ;[1 1 1] Jump via spacebar for pc testing only/ flatground tricks happen via analog stick gestures (in cpp file)
  (:Pressed
    (bind _asskate_character_movement_component (Utilities|Casting|CastToSkateCharacterMovementComponent _charactermovement))
    (if (Class|SkateCharacterMovementComponent|IsCustomMovementMode _asskate_character_movement_component "CMOVE_Skate")
      (Animation|Montage|PlayMontage (Variables|Character|GetMesh) "/Game/SkateAssets/Animations/SkateOllie_Montage.SkateOllie_Montage"
        (:then
          (Physics|AddImpulse _charactermovement (* (Math|Vector|GetUpVector (Variables|Default|GetCapsuleComponent)) 7e+02) true))))))

(event Input|KeyboardEvents|R
  (params (Key :type Key%20Structure :default "None"))
  ;[1 1 1] RESET
  (:Pressed
    (bind _returnvalue (Game|GetCurrentLevelName true))
    (Game|OpenLevel(byName) (Utilities|String|StringToName _returnvalue))))

(event Input|KeyboardEvents|F
  (params (Key :type Key%20Structure :default "None"))
  (bind _returnvalue (Transformation|GetActorRotation))
  (:Pressed
    (Transformation|SetActorRotation (Math|Rotator|MakeRotator (.roll _returnvalue) (.pitch _returnvalue) (+ (.yaw _returnvalue) 1.8e+02)))))

(event Input|KeyboardEvents|G
  (params (Key :type Key%20Structure :default "None"))
  ;[1 1 1] L/R Grabs
  (:Pressed
    (Variables|Grabs|SetisRightGrab true)
    (Class|SkateCharacter|Grab :!label _label))
  (:Released
    (Variables|Grabs|SetisRightGrab false)
    (goto _label)))

(event Input|GamepadEvents|GamepadRightTrigger
  (params (Key :type Key%20Structure :default "None"))
  ;[1 1 1] L/R Grabs
  (:Pressed
    (Variables|Grabs|SetisRightGrab true)
    (Class|SkateCharacter|Grab :!label _label))
  (:Released
    (Variables|Grabs|SetisRightGrab false)
    (goto _label)))

(event Input|GamepadEvents|GamepadLeftTrigger
  (params (Key :type Key%20Structure :default "None"))
  ;[1 1 1] Jump via spacebar for pc testing only/ flatground tricks happen via analog stick gestures (in cpp file)
  (:Pressed
    (Variables|Grabs|SetisLeftGrab true)
    (Class|SkateCharacter|Grab :!label _label))
  (:Released
    (Variables|Grabs|SetisLeftGrab false)
    (goto _label)))

(fn ConstructionScript)

(fn AlignCamerawithMoveDirection
  (Transformation|SetRelativeRotation (Variables|Default|GetCameraBoom) (Math|Rotator|MakeRotator 0.0 0.0 (.Yaw (Math|Vector|GetYawPitchfromVector (/ (- (Transformation|GetActorLocation) (Variables|Default|GetPreviousPosition)) (Utilities|Time|GetWorldDeltaSeconds))))) false false)
  (Variables|Default|SetPreviousPosition (Transformation|GetActorLocation)))