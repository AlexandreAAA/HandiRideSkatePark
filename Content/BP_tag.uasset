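; BP_tag is a tag spot whose decal the player reveals by pressing E nearby.
; The decal starts hidden, and a sphere trigger sets CanShowTag while a BP_MamieWheelChair overlaps it.
; Pressing E while that flag is set shows the decal, which is never hidden again, and debug strings report key and range changes.
; The construction script sizes the trigger from PlayerTriggerRadius.
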(event OnComponentBeginOverlap(Player_trigger)
  (params (OverlappedComponent :type Primitive%20Component%20Object%20Reference) (OtherActor :type Actor%20Object%20Reference) (OtherComp :type Primitive%20Component%20Object%20Reference) (OtherBodyIndex :type Integer) (bFromSweep :type Boolean) (SweepResult :type Hit%20Result%20Structure%20%28by%20ref%29))
  (Utilities|Casting|CastToBP_MamieWheelChair OtherActor)
  (Variables|Default|SetCanShowTag true)
  (Development|PrintString "You can tag"))

(event OnComponentEndOverlap(Player_trigger)
  (params (OverlappedComponent :type Primitive%20Component%20Object%20Reference) (OtherActor :type Actor%20Object%20Reference) (OtherComp :type Primitive%20Component%20Object%20Reference) (OtherBodyIndex :type Integer))
  (Utilities|Casting|CastToBP_MamieWheelChair OtherActor)
  (Variables|Default|SetCanShowTag false)
  (Development|PrintString "You can no longer tag"))

(event EventBeginPlay
  (Development|SetHiddeninGame (Variables|Default|GetDecal) true false))

(event Collision|EventActorBeginOverlap
  (params (OtherActor :type Actor%20Object%20Reference)))

(event EventTick
  (params (DeltaSeconds :type Float%20%28single-precision%29)))

(event Input|KeyboardEvents|E
  (params (Key :type Key%20Structure :default "None"))
  (:Pressed
    (Development|PrintString "E IS PRESSED")
    (if (Variables|Default|GetCanShowTag)
      (Development|SetHiddeninGame (Variables|Default|GetDecal) false false))))

(fn ConstructionScript
  (Components|Sphere|SetSphereRadius (Variables|Default|GetPlayer_trigger) (Variables|Default|GetPlayerTriggerRadius) true))