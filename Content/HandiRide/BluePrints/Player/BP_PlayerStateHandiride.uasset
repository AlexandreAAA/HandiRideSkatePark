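; BP_PlayerStateHandiride is a player state Blueprint for HandiRide that tallies an array of boolean tags.
; Each Tick adds the true entries of Tag1 to TagOk and prints the total when it equals the array length.
; TagOk is never reset in this graph, so the tally accumulates across frames.
; CheckTagStatus, BeginPlay and the construction script are empty.
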(event Custom|CheckTagStatus
  (params (NewParam :type Array%20of%20Booleans)))

(event EventBeginPlay)

(event EventTick
  (params (DeltaSeconds :type Float%20%28single-precision%29))
  (bind _output_get (Variables|Default|SetTag1 (Variables|Default|GetTag1)))
  (for _array_element _output_get
    (if _array_element
      (Variables|Default|SetTagOk (+ (Variables|Default|GetTagOk) 1))))
  (if (== (Variables|Default|GetTagOk) (Utilities|Array|Length (Variables|Default|GetTag1)))
    (Development|PrintString (Utilities|String|ToString(Integer) (Variables|Default|GetTagOk)))))

(fn ConstructionScript)