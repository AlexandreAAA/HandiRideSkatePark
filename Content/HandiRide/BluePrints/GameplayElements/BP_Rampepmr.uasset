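; BP_Rampepmr is a ramp actor that starts hidden in game and appears once all its linked BPTag objects are activated.
; Each tick, it counts newly activated tags, flagging each as already active, and unhides itself when the count matches the array length.
; A sphere trigger pauses this check while BP_MamieWheelChair overlaps it, so the ramp is not revealed with the wheelchair nearby.
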(event OnComponentBeginOverlap(Sphere)
  (params (OverlappedComponent :type Primitive%20Component%20Object%20Reference) (OtherActor :type Actor%20Object%20Reference) (OtherComp :type Primitive%20Component%20Object%20Reference) (OtherBodyIndex :type Integer) (bFromSweep :type Boolean) (SweepResult :type Hit%20Result%20Structure%20%28by%20ref%29))
  ;[1 1 1] change if nearby
  (Utilities|Casting|CastToBP_MamieWheelChair OtherActor)
  (bind _output_get (Variables|Default|Setis%20overlap true)))

(event OnComponentEndOverlap(Sphere)
  (params (OverlappedComponent :type Primitive%20Component%20Object%20Reference) (OtherActor :type Actor%20Object%20Reference) (OtherComp :type Primitive%20Component%20Object%20Reference) (OtherBodyIndex :type Integer))
  ;[1 1 1] change if nearby
  (Utilities|Casting|CastToBP_MamieWheelChair OtherActor)
  (Variables|Default|Setis%20overlap false))

(event EventBeginPlay
  (Rendering|SetActorHiddenInGame true))

(event Collision|EventActorBeginOverlap
  (params (OtherActor :type Actor%20Object%20Reference))
  ;[1 1 1] change if nearby
)

(event EventTick
  (params (DeltaSeconds :type Float%20%28single-precision%29))
  ;[1 1 1] change if nearby
  (if (not (stale OnComponentBeginOverlap(Sphere) _output_get))
    (for _array_element (Variables|Default|GetBP%20tag)
      (if (not (Variables|/Game/HandiRide/BluePrints/Tags/BP_TAG.BP_TAG_C|Getis_already_active _array_element))
        (if (Variables|/Game/HandiRide/BluePrints/Tags/BP_TAG.BP_TAG_C|GetActivated _array_element)
          (bind _output_get (Variables|Default|SetTag_count (+ (Variables|Default|GetTag_count) 1)))
          (Variables|/Game/HandiRide/BluePrints/Tags/BP_TAG.BP_TAG_C|Setis_already_active _array_element true)
          (Development|PrintString (Utilities|String|ToString(Integer) _output_get)))))
    (if (== (Variables|Default|GetTag_count) (Utilities|Array|Length (Variables|Default|GetBP%20tag)))
      (CallFunction|Activate))))

(fn ConstructionScript)

(fn Activate
  (Rendering|SetActorHiddenInGame false))