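; BP_TAG is a tag spot that the wheelchair player (BP_MamieWheelChair) activates by pressing T while in range.
; An INFOTAG marker spins on Tick and swaps material while the player overlaps the trigger sphere, whose radius is set in the construction script.
; Tagging reveals the decal, hides the marker and sets Activated.
; The score-adding and debug print nodes are disconnected and never run.
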(event OnComponentBeginOverlap(Player_trigger)
  (params (OverlappedComponent :type Primitive%20Component%20Object%20Reference) (OtherActor :type Actor%20Object%20Reference) (OtherComp :type Primitive%20Component%20Object%20Reference) (OtherBodyIndex :type Integer) (bFromSweep :type Boolean) (SweepResult :type Hit%20Result%20Structure%20%28by%20ref%29))
  ;[1 1 1] Detect if Playable character is overlapping / can tag
  (Utilities|Casting|CastToBP_MamieWheelChair OtherActor)
  (Variables|Default|SetOverlaps true)
  (Rendering|Material|SetMaterial (Variables|Default|GetINFOTAG) 0 "/Game/HandiRide/Material_Instance/Mi_TAG_POSSIBLE.Mi_TAG_POSSIBLE"))

(event OnComponentEndOverlap(Player_trigger)
  (params (OverlappedComponent :type Primitive%20Component%20Object%20Reference) (OtherActor :type Actor%20Object%20Reference) (OtherComp :type Primitive%20Component%20Object%20Reference) (OtherBodyIndex :type Integer))
  ;[1 1 1] Detect if Playable character is overlapping / can tag
  (Utilities|Casting|CastToBP_MamieWheelChair OtherActor)
  (Variables|Default|SetOverlaps false)
  (Rendering|Material|SetMaterial (Variables|Default|GetINFOTAG) 0 "/Game/HandiRide/Material_Instance/Mi_Traffiv_Cone.Mi_Traffiv_Cone"))

(event EventBeginPlay
  (Variables|Default|SetActivated false))

(event Collision|EventActorBeginOverlap
  (params (OtherActor :type Actor%20Object%20Reference)))

(event EventTick
  (params (DeltaSeconds :type Float%20%28single-precision%29))
  (bind _infotag (Variables|Default|GetINFOTAG))
  ;[1 1 1] Infotag - Rotation
  (Transformation|SetRelativeRotation _infotag (Math|Rotator|MakeRotator 0.0 0.0 (+ (.yaw (Variables|/Script/Engine.SceneComponent|GetRelativeRotation _infotag)) 1.5)) false false))

(event Input|KeyboardEvents|T
  (params (Key :type Key%20Structure :default "None"))
  ;[1 1 1] Tag - on button press
  (:Pressed
    (if (Variables|Default|GetOverlaps)
      (Rendering|SetVisibility (Variables|Default|GetDecal) true false)
      (Rendering|SetVisibility (Variables|Default|GetINFOTAG) false false)
      (Variables|Default|SetActivated true))))

(fn ConstructionScript
  (Components|Sphere|SetSphereRadius (Variables|Default|GetPlayer_trigger) (Variables|Default|GetPlayerTriggerRadius) true))