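; BP_Checker is an actor that watches a collection of tags and activates a target once all of them are activated.
; Each Tick until it fires, it counts the activated entries in TagsCollection and compares the count to the collection's length.
; On a match it sets IsActive, which stops further checks, and calls Activate on ToActivate.
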(event EventBeginPlay)

(event Collision|EventActorBeginOverlap
  (params (OtherActor :type Actor%20Object%20Reference)))

(event EventTick
  (params (DeltaSeconds :type Float%20%28single-precision%29))
  (if (not (Variables|Default|Getis_active))
    (bind _output (CallFunction|CheckifAllTagsActive))
    (if _output
      (Variables|Default|Setis_active true)
      (CallFunction|ActivateStuff))))

(fn ConstructionScript)

(fn CheckifAllTagsActive
  (for _array_element (Variables|Default|GetTags_Collection)
    (if (Variables|/Game/HandiRide/BluePrints/Tags/BP_TAG.BP_TAG_C|GetActivated _array_element)
      (LocalVariables|SetTag_active_count (+ (LocalVariables|GetTag_active_count) 1))))
  (if (== (LocalVariables|GetTag_active_count) (Utilities|Array|Length (Variables|Default|GetTags_Collection)))
    (return true)
    (else
      (return false))))

(fn ActivateStuff
  (Default|Activate (Variables|Default|GetToActivate)))